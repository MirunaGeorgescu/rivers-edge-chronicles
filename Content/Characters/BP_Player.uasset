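; BP_Player is the player Blueprint, handling basic movement and mouse-look through input axis events.
; Forward/backward movement follows control yaw only, while right/left movement derives its direction from control yaw and roll, so pitch affects neither.
; Mouse axes feed directly into controller pitch and yaw input, and the construction script is empty.
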(event Input|AxisEvents|InputAxisMoveRight/Left
  (params (AxisValue :type Float%20%28single-precision%29))
  (bind _returnvalue (Pawn|GetControlRotation :!class /Script/Engine.Pawn))
  ;[0.1597 0.1597 0.1597] Character Movement
  ;;[0 0 0] Right/Left Movement
  (Pawn|Input|AddMovementInput (Math|Vector|GetRightVector (Math|Rotator|MakeRotator (.roll _returnvalue) 0.0 (.yaw _returnvalue))) AxisValue false))

(event Input|AxisEvents|InputAxisMoveForward/Backward
  (params (AxisValue :type Float%20%28single-precision%29))
  ;[0.1597 0.1597 0.1597] Character Movement
  ;;[0 0 0] Forward/Backward Movement
  (Pawn|Input|AddMovementInput (Math|Vector|GetForwardVector (Math|Rotator|MakeRotator 0.0 0.0 (.yaw (Pawn|GetControlRotation :!class /Script/Engine.Pawn)))) AxisValue false))

(event Input|AxisEvents|InputAxisMouseUp/Down
  (params (AxisValue :type Float%20%28single-precision%29))
  ;[0.1875 0.1875 0.1875] Camera Movement
  ;;[0 0 0] Up/Down Movement
  (Pawn|Input|AddControllerPitchInput AxisValue))

(event Input|AxisEvents|InputAxisMouseRight/Left
  (params (AxisValue :type Float%20%28single-precision%29))
  ;[0.1875 0.1875 0.1875] Camera Movement
  ;;[0 0 0] Right/Left Movement
  (Pawn|Input|AddControllerYawInput AxisValue))

(fn ConstructionScript)